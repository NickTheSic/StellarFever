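; BP_AmmoBay is an ammo bay that displays its remaining refills on a widget component.
; Every Tick it casts the ReserveComp widget to UI_AmmoBay and pushes RefillsAllowed and MaxedRefills into the ammo bar.
; It also sets the widget's Hide flag when the player pawn is more than 500 units away.
; The graph only drives the display and contains no refill logic.
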(event EventBeginPlay)

(event Collision|EventActorBeginOverlap
  (params (OtherActor :type Actor%20Object%20Reference)))

(event EventTick
  (params (DeltaSeconds :type Float%20%28single-precision%29))
  (bind _maxedrefills (Variables|Default|GetMaxedRefills))
  (bind _refillsallowed (Variables|Default|GetRefillsAllowed))
  (bind _asui_ammo_bay (Utilities|Casting|CastToUI_AmmoBay (UserInterface|GetUserWidgetObject (Variables|Default|GetReserveComp))))
  (bind _output_get (Variables|Default|SetAmmoBarWidget _asui_ammo_bay))
  (Utilities|FlowControl|Sequence
    (:then_0
      (Variables|/Game/AdrianFolder/UI_AmmoBay.UI_AmmoBay_C|SetCurrentAmmo _output_get _refillsallowed)
      (Variables|/Game/AdrianFolder/UI_AmmoBay.UI_AmmoBay_C|SetReserveAmmo _output_get _maxedrefills))
    (:then_1
      (Default|UpdateAmmoBar _output_get (Math|Conversions|ToFloat(Integer) _refillsallowed) (Math|Conversions|ToFloat(Integer) _maxedrefills)))
    (:then_2
      (if (> (Transformation|GetDistanceTo (Game|Player|GetPlayerPawn 0)) 5e+02)
        (Variables|/Game/AdrianFolder/UI_AmmoBay.UI_AmmoBay_C|SetHide (Variables|Default|GetAmmoBarWidget) true)
        (else
          (Variables|/Game/AdrianFolder/UI_AmmoBay.UI_AmmoBay_C|SetHide (Variables|Default|GetAmmoBarWidget) false))))))

(fn ConstructionScript)