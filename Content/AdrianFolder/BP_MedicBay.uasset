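; BP_MedicBay is a medic bay actor that displays its remaining healing reserve through a UI_MedicBay widget on its ReserveComp component.
; Every Tick it casts that widget, copies HealAvailable and IDefaultHealthAvailable into it as current and reserve health, and refreshes the bar.
; It also toggles the widget's Hide flag by player pawn distance, hiding it when the player is far away.
; The graphs shown contain no healing logic.
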(event EventBeginPlay)

(event Collision|EventActorBeginOverlap
  (params (OtherActor :type Actor%20Object%20Reference)))

(event EventTick
  (params (DeltaSeconds :type Float%20%28single-precision%29))
  (bind _healavailable (Variables|Default|GetHealAvailable))
  (bind _idefaulthealthavailable (Variables|Default|GetiDefaultHealthAvailable))
  (bind _asui_medic_bay (Utilities|Casting|CastToUI_MedicBay (UserInterface|GetUserWidgetObject (Variables|Default|GetReserveComp))))
  (bind _output_get (Variables|Default|SetHealthBarWidget _asui_medic_bay))
  (Utilities|FlowControl|Sequence
    (:then_0
      (Variables|/Game/AdrianFolder/UI_MedicBay.UI_MedicBay_C|SetCurrentHealth _output_get _healavailable)
      (Variables|/Game/AdrianFolder/UI_MedicBay.UI_MedicBay_C|SetReserveHealth _output_get _idefaulthealthavailable))
    (:then_1
      (Default|UpdateHealthBar _output_get (Math|Conversions|ToFloat(Integer) _healavailable) (Math|Conversions|ToFloat(Integer) _idefaulthealthavailable)))
    (:then_2
      (if (> (Transformation|GetDistanceTo (Game|Player|GetPlayerPawn 0)) 5e+02)
        (Variables|/Game/AdrianFolder/UI_MedicBay.UI_MedicBay_C|SetHide (Variables|Default|GetHealthBarWidget) true)
        (else
          (Variables|/Game/AdrianFolder/UI_MedicBay.UI_MedicBay_C|SetHide (Variables|Default|GetHealthBarWidget) false))))))

(fn ConstructionScript)