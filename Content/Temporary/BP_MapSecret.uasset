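; BP_MapSecret is a single-player map secret that opens a door and teleporter once its eleven buttons are pressed.
; A once-per-second tick counts inactive buttons as pressed and shows progress through a dynamic material's Angle on a plane.
; Completion shifts the door, enables the teleport box, whose overlap loads Launch_Room, and stops ticking.
; In other game modes, BeginPlay destroys the buttons and disables tick.
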(event OnComponentBeginOverlap(teleportbox)
  (params (OverlappedComponent :type Primitive%20Component%20Object%20Reference) (OtherActor :type Actor%20Object%20Reference) (OtherComp :type Primitive%20Component%20Object%20Reference) (OtherBodyIndex :type Integer) (bFromSweep :type Boolean) (SweepResult :type Hit%20Result%20Structure%20%28by%20ref%29))
  (Game|OpenLevel(byName) "Launch_Room"))

(event EventBeginPlay
  (bind _plane (Variables|Default|GetPlane))
  (if (!= (Utilities|GetClass (Game|GetGameMode)) "/Game/Blueprints/BP_SinglePlayerGameMode.BP_SinglePlayerGameMode_C")
    (for _array_element (Variables|Default|GetButtonsList)
      (Actor|DestroyActor _array_element)
      (Actor|Tick|SetActorTickEnabled false))
    (else
      (Actor|Tick|SetActorTickInterval 1.0)
      (bind _returnvalue (Rendering|Material|CreateDynamicMaterialInstance _plane 0 (Rendering|Material|GetMaterial _plane 0) "None" :!class /Script/Engine.PrimitiveComponent))
      (Rendering|Material|SetVectorParameterValue _returnvalue "Color" "(R=0.000000,G=0.834787,B=1.000000,A=1.000000)" :!class /Script/Engine.MaterialInstanceDynamic))))

(event EventTick
  (params (DeltaSeconds :type Float%20%28single-precision%29))
  (bind _door (Variables|Default|GetDoor))
  (bind _all_pressed (CallFunction|CheckIsAllPressed))
  (Rendering|Material|SetScalarParameterValue (stale EventBeginPlay _returnvalue) "Angle" (Math|Conversions|ToFloat(Integer) (/ (* (Variables|Default|GetiNumberPressed) 360) 11)) :!class /Script/Engine.MaterialInstanceDynamic)
  (if _all_pressed
    (if (not (Variables|Default|GetHasMovedDoor))
      (Variables|Default|SetHasMovedDoor true)
      (Transformation|SetActorLocation _door (+ (Transformation|GetActorLocation _door) "0,170.000000, 0") false false)
      (Collision|SetCollisionEnabled (Variables|Default|Getteleportbox) "QueryAndPhysics")
      (Actor|Tick|SetActorTickEnabled false))))

(fn ConstructionScript)

(fn CheckIsAllPressed
  (Variables|Default|SetiNumberPressed 0)
  (for _array_element (Variables|Default|GetButtonsList)
    (if (not (Math|Boolean|Equal(Boolean) (Variables|/Script/StellarFever.BaseEvent|GetbIsActive _array_element) true))
      (Math|Integer|IncrementInt (Variables|Default|GetiNumberPressed))))
  (return (== (Variables|Default|GetiNumberPressed) 11)))