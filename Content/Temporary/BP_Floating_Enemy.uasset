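; BP_Floating_Enemy is an actor Blueprint that gives an enemy an idle floating motion, with no combat or AI logic.
; It caches its spawn location on BeginPlay, then each Tick offsets Z from that point by a cosine of game time to bob vertically.
; Tick also applies a slow, delta-time-scaled yaw spin, and both movements run without sweep collision.
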(event EventBeginPlay
  (bind _output_get (Variables|Default|SetStartPos (Transformation|GetActorLocation))))

(event EventTick
  (params (DeltaSeconds :type Float%20%28single-precision%29))
  (Transformation|SetActorLocation (+ (stale EventBeginPlay _output_get) (Math|Vector|MakeVector 0.0 0.0 (* (Math|Trig|Cos(Radians) (Utilities|Time|GetTimeSeconds)) 6e+01))) false false)
  (Class|Actor|AddActorWorldRotation (Math|Rotator|MakeRotator 0.0 0.0 (* (Utilities|Time|GetWorldDeltaSeconds) -5.0))))

(fn ConstructionScript)