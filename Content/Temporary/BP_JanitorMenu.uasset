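; BP_JanitorMenu is a janitor actor, apparently for the menu scene, that walks a looping patrol through a list of waypoint actors.
; Each Tick it moves toward the current point at constant speed along a flattened, normalized direction, without sweep or navigation.
; Within a small squared-distance threshold it advances the index, wrapping at the end, and snaps the skeletal mesh's yaw toward the next point using Atan2.
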(event EventBeginPlay)

(event Collision|EventActorBeginOverlap
  (params (OtherActor :type Actor%20Object%20Reference)))

(event EventTick
  (params (DeltaSeconds :type Float%20%28single-precision%29))
  (bind _returnvalue (Transformation|GetActorLocation))
  (if (< (Class|KismetMathLibrary|VectorDistanceSquared _returnvalue (Transformation|GetActorLocation (Utilities|Array|Get(acopy) (Variables|Default|GetInAIPoints) (Variables|Default|GetiPoint)))) 2.5e+03)
    (bind _output_get (Variables|Default|SetiPoint (+ (Variables|Default|GetiPoint) 1)))
    (if (>= _output_get (Utilities|Array|Length (Variables|Default|GetInAIPoints)))
      (Variables|Default|SetiPoint 0))
    (Transformation|SetWorldRotation (Variables|Default|GetSkeletalMesh) (Math|Rotator|MakeRotator 0.0 0.0 (Class|KismetMathLibrary|DegAtan2 (* (.X (Math|Vector|BreakVector (Math|Vector|Normalize (* (- (Transformation|GetActorLocation (Utilities|Array|Get(acopy) (Variables|Default|GetInAIPoints) (Variables|Default|GetiPoint))) _returnvalue) "1.000000,1.000000,0.000000")))) -1.0) (.Y (Math|Vector|BreakVector (Math|Vector|Normalize (* (- (Transformation|GetActorLocation (Utilities|Array|Get(acopy) (Variables|Default|GetInAIPoints) (Variables|Default|GetiPoint))) _returnvalue) "1.000000,1.000000,0.000000")))))) false false)
    (else
      (Transformation|SetActorLocation (+ (Transformation|GetActorLocation) (* (* (Math|Vector|Normalize (* (- (Transformation|GetActorLocation (Utilities|Array|Get(acopy) (Variables|Default|GetInAIPoints) (Variables|Default|GetiPoint))) _returnvalue) "1.000000,1.000000,0.000000")) (Utilities|Time|GetWorldDeltaSeconds)) 2.5e+02)) false false))))

(fn ConstructionScript)