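; BP_DoorObject is a door actor whose behavior and indicator lights are driven by the UcDoorStatus value.
; Every Tick it colors two point lights red for status 4, presumably locked, and green otherwise.
; Two transient states each play their own actor sequence, likely open and close, then advance to a resting state after a short Delay.
; The graph polls the status rather than reacting to overlaps, which are empty.
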(event EventBeginPlay)

(event Collision|EventActorBeginOverlap
  (params (OtherActor :type Actor%20Object%20Reference)))

(event EventTick
  (params (DeltaSeconds :type Float%20%28single-precision%29))
  (bind _returnvalue (Math|Color|MakeColor 1.0 0.0 0.0))
  (bind _returnvalue_2 (Math|Color|MakeColor 0.0 1.0 0.0))
  (if (== (Variables|Default|GetucDoorStatus) 4)
    (Rendering|Components|Light|SetLightColor (Variables|Default|GetPointLight1) _returnvalue true)
    (Rendering|Components|Light|SetLightColor (Variables|Default|GetPointLight) _returnvalue true)
    (else
      (Rendering|Components|Light|SetLightColor (Variables|Default|GetPointLight1) _returnvalue_2 true)
      (Rendering|Components|Light|SetLightColor (Variables|Default|GetPointLight) _returnvalue_2 true)))
  (if (== (Variables|Default|GetucDoorStatus) 1)
    (Sequencer|Player|Play (Variables|/Script/ActorSequence.ActorSequenceComponent|GetSequencePlayer (Variables|Default|GetActorSequence)) :!class /Script/MovieScene.MovieSceneSequencePlayer)
    (Utilities|FlowControl|Delay 1.0)
    (Variables|Default|SetucDoorStatus 2)
    (elif (== (Variables|Default|GetucDoorStatus) 3)
      (Sequencer|Player|Play (Variables|/Script/ActorSequence.ActorSequenceComponent|GetSequencePlayer (Variables|Default|GetActorSequence2)) :!class /Script/MovieScene.MovieSceneSequencePlayer)
      (Utilities|FlowControl|Delay 1.0)
      (Variables|Default|SetucDoorStatus 0))))

(event Collision|EventActorEndOverlap
  (params (OtherActor :type Actor%20Object%20Reference)))

(fn ConstructionScript)