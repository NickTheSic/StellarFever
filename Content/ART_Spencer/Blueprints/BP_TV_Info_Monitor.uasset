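; TV info monitor prop with selectable stand meshes: basic base, jetpack, propeller, two wall arms or wheel base.
; ShowCorrectStands hides all stands, then shows the first one flagged by its booleans, brightening two rect lights for the jetpack.
; Unwired EventGraph fragments hold duplicate selection logic, timeline-driven vertical movement and propeller rotation.
; BeginPlay, Tick and the Construction Script are empty, so none of this logic runs by itself.
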(event EventBeginPlay)

(event Collision|EventActorBeginOverlap
  (params (OtherActor :type Actor%20Object%20Reference)))

(event EventTick
  (params (DeltaSeconds :type Float%20%28single-precision%29)))

(fn ConstructionScript)

(fn HideAllStands
  (Rendering|SetVisibility (Variables|Default|GetSTM_TV_JetPack) false false))

(fn ShowCorrectStands
  (CallFunction|HideAllStands)
  (if (Variables|Default|GetBasic_Base)
    (Rendering|SetVisibility (Variables|Default|GetSTM_TV_BasicBase) true false)
    (elif (Variables|Default|GetJet_Pack)
      (Rendering|SetVisibility (Variables|Default|GetSTM_TV_JetPack) true false)
      (Rendering|Components|Light|SetIntensity (Variables|Default|GetRectLight) 2e+03)
      (elif (Variables|Default|GetPropeller)
        (Rendering|SetVisibility (Variables|Default|GetSTM_TV_Propeller) true false)
        (elif (Variables|Default|GetWall_Arm_1)
          (Rendering|SetVisibility (Variables|Default|GetSTM_TV_WallArm1a) true true)
          (elif (Variables|Default|GetWall_Arm_2)
            (Rendering|SetVisibility (Variables|Default|GetSTM_TV_Wall_Arm_2) true false)
            (elif (Variables|Default|GetWheel_Base)
              (Rendering|SetVisibility (Variables|Default|GetSTM_TV_WheelBase) true true))))))))