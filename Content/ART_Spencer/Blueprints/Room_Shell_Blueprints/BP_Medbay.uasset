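; Medbay room shell Blueprint that, when flagged as a tutorial instance, drives a time-based material effect on its ceilings and walls.
; On BeginPlay it creates and stores dynamic material instances for two ceiling meshes and the wall mesh.
; The first Pawn to overlap the MaterialLoad trigger records a start time.
; Tick then feeds the elapsed seconds into each material's TimeIn parameter every frame.
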(event OnComponentBeginOverlap(MaterialLoad)
  (params (OverlappedComponent :type Primitive%20Component%20Object%20Reference) (OtherActor :type Actor%20Object%20Reference) (OtherComp :type Primitive%20Component%20Object%20Reference) (OtherBodyIndex :type Integer) (bFromSweep :type Boolean) (SweepResult :type Hit%20Result%20Structure%20%28by%20ref%29))
  (if (Variables|Default|GetTutorialInstance)
    (if (not (Variables|Default|GetHasMaterialBeenInstantiated))
      (Utilities|Casting|CastToPawn OtherActor)
      (Variables|Default|SetHasMaterialBeenInstantiated true)
      (Variables|Default|SetSecondsOffset (Utilities|Time|GetGameTimeinSeconds)))))

(event EventBeginPlay
  (bind _stm_medbay_medbay_ceiling (Variables|Default|GetSTM_Medbay_Medbay_Ceiling))
  (bind _stm_medbay_medbay_ceiling1 (Variables|Default|GetSTM_Medbay_Medbay_Ceiling1))
  (bind _stm_medbay_medbay_walls (Variables|Default|GetSTM_Medbay_Medbay_walls))
  (if (Variables|Default|GetTutorialInstance)
    (for (_array_element _array_index) (Rendering|Material|GetMaterials _stm_medbay_medbay_ceiling)
      (bind _returnvalue (Rendering|Material|CreateDynamicMaterialInstance _stm_medbay_medbay_ceiling _array_index _array_element "None" :!class /Script/Engine.PrimitiveComponent))
      (Utilities|Array|Add (Variables|Default|GetDynamicMaterials) _returnvalue))
    (for (_array_element_2 _array_index_2) (Rendering|Material|GetMaterials _stm_medbay_medbay_ceiling1)
      (bind _returnvalue_2 (Rendering|Material|CreateDynamicMaterialInstance _stm_medbay_medbay_ceiling1 _array_index_2 _array_element_2 "None" :!class /Script/Engine.PrimitiveComponent))
      (Utilities|Array|Add (Variables|Default|GetDynamicMaterials) _returnvalue_2))
    (for (_array_element_3 _array_index_3) (Rendering|Material|GetMaterials _stm_medbay_medbay_walls)
      (bind _returnvalue_3 (Rendering|Material|CreateDynamicMaterialInstance _stm_medbay_medbay_walls _array_index_3 _array_element_3 "None" :!class /Script/Engine.PrimitiveComponent))
      (Utilities|Array|Add (Variables|Default|GetDynamicMaterials) _returnvalue_3))))

(event EventTick
  (params (DeltaSeconds :type Float%20%28single-precision%29))
  (if (Variables|Default|GetTutorialInstance)
    (if (Variables|Default|GetHasMaterialBeenInstantiated)
      (for _array_element (Variables|Default|GetDynamicMaterials)
        (Rendering|Material|SetScalarParameterValue _array_element "TimeIn" (- (Utilities|Time|GetGameTimeinSeconds) (Variables|Default|GetSecondsOffset)) :!class /Script/Engine.MaterialInstanceDynamic)))))

(fn ConstructionScript)