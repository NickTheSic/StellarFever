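; BP_Radio is an interactable radio that plays a random music track when the player presses E nearby.
; BeginPlay fills a song bank from its cue variables, and the Input_detector overlap enables or disables input for player controller 0.
; The first E release only sets a Start flag.
; Later releases flip-flop between playing a randomly picked song and stopping the current one.
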(event OnComponentBeginOverlap(input_detector)
  (params (OverlappedComponent :type Primitive%20Component%20Object%20Reference) (OtherActor :type Actor%20Object%20Reference) (OtherComp :type Primitive%20Component%20Object%20Reference) (OtherBodyIndex :type Integer) (bFromSweep :type Boolean) (SweepResult :type Hit%20Result%20Structure%20%28by%20ref%29))
  ;[1 1 1] Input Enabler
  (Input|EnableInput (Game|GetPlayerController 0)))

(event OnComponentEndOverlap(input_detector)
  (params (OverlappedComponent :type Primitive%20Component%20Object%20Reference) (OtherActor :type Actor%20Object%20Reference) (OtherComp :type Primitive%20Component%20Object%20Reference) (OtherBodyIndex :type Integer))
  ;[1 1 1] Input Enabler
  (Input|DisableInput (Game|GetPlayerController 0)))

(event EventBeginPlay
  ;[1 1 1] Song Array
  (Variables|Default|SetSong%20Bank (Utilities|Array|MakeArray (Variables|Default|Gettrying_to_remember-melodic_pictures_01_Cue) (Variables|Default|Getpeace__60_sec-rick_dickert_01_Cue) (Variables|Default|Getroyal_york_cello_theme-rick_dickert_01_Cue) (Variables|Default|Getsnowflake_-_Ethereal_Space_01_Cue) (Variables|Default|Getteru_-_Goodbye_War_Hello_Peace_01_Cue) (Variables|Default|Getmeadow-enrico_altavilla_01_Cue) (Variables|Default|Getlife_in_a_day-enrico_altavilla_01_Cue) (Variables|Default|GetAlexBeroza_-_Improvisation_On_Friday____01_Cue) (Variables|Default|Getcdk_-_Silence_Await_01_Cue) (Variables|Default|GetPOL-moonlight-short_Cue))))

(event Input|KeyboardEvents|E
  (params (Key :type Key%20Structure))
  (:Released
    (if (Variables|Default|GetStart)
      (Utilities|FlowControl|FlipFlop
        (:A
          (bind _output_get (Variables|Default|SetRandomizer (Math|Random|RandomInteger (Utilities|Array|Length (Variables|Default|GetSong%20Bank)))))
          (bind _output_get_2 (Variables|Default|SetCurrentSong (Utilities|Array|Get(acopy) (Variables|Default|GetSong%20Bank) _output_get)))
          (Audio|Components|Audio|Play _output_get_2 0.0))
        (:B
          (Audio|Components|Audio|Stop (Variables|Default|GetCurrentSong))))
      (else
        (Variables|Default|SetStart true)))))

(fn ConstructionScript)