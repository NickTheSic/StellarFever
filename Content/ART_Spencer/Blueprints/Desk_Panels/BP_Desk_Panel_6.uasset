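; Desk panel prop with red, blue and green bulb screens that mirror the state of its panel light child actors.
; Every Tick, one function per color casts its child actor to the matching panel light Blueprint and reads its light visibility.
; Each then sets that screen mesh's material to the colored bulb or the shared off material, polling continuously rather than reacting to events.
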(event EventBeginPlay)

(event Collision|EventActorBeginOverlap
  (params (OtherActor :type Actor%20Object%20Reference)))

(event EventTick
  (params (DeltaSeconds :type Float%20%28single-precision%29))
  (CallFunction|RedBulbMatChange)
  (CallFunction|BlueBulbMatChange)
  (CallFunction|GreenBulbMatChange))

(fn ConstructionScript)

(fn RedBulbMatChange
  (bind _panel_6_screen022 (Variables|Default|GetPanel_6_Screen022))
  (bind _asbp_panel_light_red (Utilities|Casting|CastToBP_Panel_Light_Red (Variables|/Script/Engine.ChildActorComponent|GetChildActor (Variables|Default|GetBP_Panel_Light_Red))))
  (bind _isvisible (Default|GetLightVisibility _asbp_panel_light_red))
  (if _isvisible
    (Rendering|Material|SetMaterial _panel_6_screen022 0 "/Game/ART_Spencer/Blueprints/Desk_Panels/MAT_Red_Bulb.MAT_Red_Bulb")
    (else
      (Rendering|Material|SetMaterial _panel_6_screen022 0 "/Game/ART_Spencer/Blueprints/Desk_Panels/Mat_Bulb_Off.MAT_Bulb_Off"))))

(fn BlueBulbMatChange
  (bind _panel_6_screen020 (Variables|Default|GetPanel_6_Screen020))
  (bind _asbp_panel_light_blue (Utilities|Casting|CastToBP_Panel_Light_Blue (Variables|/Script/Engine.ChildActorComponent|GetChildActor (Variables|Default|GetBP_Panel_Light_Blue))))
  (bind _isvisible (Default|GetLightVisibility _asbp_panel_light_blue))
  (if _isvisible
    (Rendering|Material|SetMaterial _panel_6_screen020 0 "/Game/ART_Spencer/Blueprints/Desk_Panels/MAT_Blue_Bulb.MAT_Blue_Bulb")
    (else
      (Rendering|Material|SetMaterial _panel_6_screen020 0 "/Game/ART_Spencer/Blueprints/Desk_Panels/Mat_Bulb_Off.MAT_Bulb_Off"))))

(fn GreenBulbMatChange
  (bind _panel_6_screen021 (Variables|Default|GetPanel_6_Screen021))
  (bind _asbp_panel_light_green (Utilities|Casting|CastToBP_Panel_Light_Green (Variables|/Script/Engine.ChildActorComponent|GetChildActor (Variables|Default|GetBP_Panel_Light_Green))))
  (bind _isvisible (Default|GetLightVisibility _asbp_panel_light_green))
  (if _isvisible
    (Rendering|Material|SetMaterial _panel_6_screen021 0 "/Game/ART_Spencer/Blueprints/Desk_Panels/MAT_Green_Bulb.MAT_Green_Bulb")
    (else
      (Rendering|Material|SetMaterial _panel_6_screen021 0 "/Game/ART_Spencer/Blueprints/Desk_Panels/Mat_Bulb_Off.MAT_Bulb_Off"))))