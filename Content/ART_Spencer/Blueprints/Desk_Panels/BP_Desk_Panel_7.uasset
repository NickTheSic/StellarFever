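; Desk panel prop with a video screen and indicator bulbs, starting on a muted logo video at BeginPlay.
; Events change to a random playlist video after a brief loading clip, toggle mute, or swap back to the off screen.
; Tick matches five bulb materials to their child light actors' visibility, except the third yellow bulb, which ignores that result and stays lit.
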(event Custom|RESET_Screens
  (Rendering|SetVisibility (Variables|Default|GetVideo%20Screen) false false)
  (Rendering|SetVisibility (Variables|Default|GetOff%20Screen) true false))

(event Custom|Toggle%20Video%20To%20Play
  (Media|MediaPlayer|OpenSource (Variables|Default|GetMediaPlayer) "/Game/ART_Spencer/Movies/Videos/SPS_Minimalist_Logo_Screen.SPS_Minimalist_Logo_Screen"))

(event Custom|Change%20Channel
  (Media|MediaPlayer|OpenSource (Variables|Default|GetMediaPlayer) "/Game/ART_Spencer/Movies/Videos/Looping_Loading_Background.Looping_Loading_Background")
  (Utilities|FlowControl|Delay 0.5)
  (bind _returnvalue (Class|MediaPlaylist|GetRandom (Variables|Default|GetVideoPlaylist)))
  (Media|MediaPlayer|OpenSource (Variables|Default|GetMediaPlayer) _returnvalue))

(event Custom|Make%20Visible%20Video%20To%20Play
  (Rendering|SetVisibility (Variables|Default|GetOff%20Screen) false false)
  (Rendering|SetVisibility (Variables|Default|GetVideo%20Screen) true false))

(event Custom|Mute%20Volume
  (Utilities|FlowControl|FlipFlop
    (:A
      (Audio|Components|Audio|SetVolumeMultiplier (Variables|Default|GetMediaSound) 1.0 :!class /Script/AudioMixer.SynthComponent))
    (:B
      (Audio|Components|Audio|SetVolumeMultiplier (Variables|Default|GetMediaSound) 0.0 :!class /Script/AudioMixer.SynthComponent))))

(event Custom|CustomEvent
  (params (DeltaSeconds :type Float%20%28single-precision%29)))

(event EventBeginPlay
  ;[1 1 1] start video muted
  (Audio|Components|Audio|SetVolumeMultiplier (Variables|Default|GetMediaSound) 0.0 :!class /Script/AudioMixer.SynthComponent)
  (CallFunction|MakeVisibleVideotoPlay)
  (CallFunction|ToggleVideotoPlay))

(event Collision|EventActorBeginOverlap
  (params (OtherActor :type Actor%20Object%20Reference)))

(event EventTick
  (params (DeltaSeconds :type Float%20%28single-precision%29))
  (CallFunction|YellowBulbMatChange)
  (CallFunction|YellowBulbMatChange1)
  (CallFunction|YellowBulbMatChange2)
  (CallFunction|RedBulbMatChange)
  (CallFunction|RedBulbMatChange1))

(fn ConstructionScript)

(fn YellowBulbMatChange
  (bind _panel_7_capsule035 (Variables|Default|GetPanel_7_Capsule035))
  (bind _asbp_panel_light_yellow (Utilities|Casting|CastToBP_Panel_Light_Yellow (Variables|/Script/Engine.ChildActorComponent|GetChildActor (Variables|Default|GetBP_Panel_Light_Yellow))))
  (bind _isvisible (Default|GetLightVisibility _asbp_panel_light_yellow))
  (if _isvisible
    (Rendering|Material|SetMaterial _panel_7_capsule035 0 "/Game/ART_Spencer/Blueprints/Desk_Panels/MAT_Yellow_Bulb.MAT_Yellow_Bulb")
    (else
      (Rendering|Material|SetMaterial _panel_7_capsule035 0 "/Game/ART_Spencer/Blueprints/Desk_Panels/Mat_Bulb_Off.MAT_Bulb_Off"))))

(fn RedBulbMatChange
  (bind _panel_7_screen018 (Variables|Default|GetPanel_7_Screen018))
  (bind _asbp_panel_light_red (Utilities|Casting|CastToBP_Panel_Light_Red (Variables|/Script/Engine.ChildActorComponent|GetChildActor (Variables|Default|GetBP_Panel_Light_Red))))
  (bind _isvisible (Default|GetLightVisibility _asbp_panel_light_red))
  (if _isvisible
    (Rendering|Material|SetMaterial _panel_7_screen018 0 "/Game/ART_Spencer/Blueprints/Desk_Panels/MAT_Red_Bulb.MAT_Red_Bulb")
    (else
      (Rendering|Material|SetMaterial _panel_7_screen018 0 "/Game/ART_Spencer/Blueprints/Desk_Panels/Mat_Bulb_Off.MAT_Bulb_Off"))))

(fn YellowBulbMatChange1
  (bind _panel_7_capsule036 (Variables|Default|GetPanel_7_Capsule036))
  (bind _asbp_panel_light_yellow (Utilities|Casting|CastToBP_Panel_Light_Yellow (Variables|/Script/Engine.ChildActorComponent|GetChildActor (Variables|Default|GetBP_Panel_Light_Yellow1))))
  (bind _isvisible (Default|GetLightVisibility _asbp_panel_light_yellow))
  (if _isvisible
    (Rendering|Material|SetMaterial _panel_7_capsule036 0 "/Game/ART_Spencer/Blueprints/Desk_Panels/MAT_Yellow_Bulb.MAT_Yellow_Bulb")
    (else
      (Rendering|Material|SetMaterial _panel_7_capsule036 0 "/Game/ART_Spencer/Blueprints/Desk_Panels/Mat_Bulb_Off.MAT_Bulb_Off"))))

(fn YellowBulbMatChange2
  (bind _panel_7_capsule037 (Variables|Default|GetPanel_7_Capsule037))
  (bind _asbp_panel_light_yellow (Utilities|Casting|CastToBP_Panel_Light_Yellow (Variables|/Script/Engine.ChildActorComponent|GetChildActor (Variables|Default|GetBP_Panel_Light_Yellow2))))
  (Default|GetLightVisibility _asbp_panel_light_yellow)
  (if true
    (Rendering|Material|SetMaterial _panel_7_capsule037 0 "/Game/ART_Spencer/Blueprints/Desk_Panels/MAT_Yellow_Bulb.MAT_Yellow_Bulb")
    (else
      (Rendering|Material|SetMaterial _panel_7_capsule037 0 "/Game/ART_Spencer/Blueprints/Desk_Panels/Mat_Bulb_Off.MAT_Bulb_Off"))))

(fn RedBulbMatChange1
  (bind _panel_7_screen019 (Variables|Default|GetPanel_7_Screen019))
  (bind _asbp_panel_light_red (Utilities|Casting|CastToBP_Panel_Light_Red (Variables|/Script/Engine.ChildActorComponent|GetChildActor (Variables|Default|GetBP_Panel_Light_Red1))))
  (bind _isvisible (Default|GetLightVisibility _asbp_panel_light_red))
  (if _isvisible
    (Rendering|Material|SetMaterial _panel_7_screen019 0 "/Game/ART_Spencer/Blueprints/Desk_Panels/MAT_Red_Bulb.MAT_Red_Bulb")
    (else
      (Rendering|Material|SetMaterial _panel_7_screen019 0 "/Game/ART_Spencer/Blueprints/Desk_Panels/Mat_Bulb_Off.MAT_Bulb_Off"))))