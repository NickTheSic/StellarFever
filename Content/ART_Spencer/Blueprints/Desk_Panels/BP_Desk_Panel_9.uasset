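; Desk panel actor with a video screen that plays looping and playlist videos through a MediaPlayer.
; BeginPlay mutes the media sound, swaps the off-screen mesh for the video screen and opens the looping loading background.
; ChangeChannel shows that loading clip for a brief delay, then opens a random VideoPlaylist entry.
; MuteVolume toggles sound through a FlipFlop, and RESET_Screens restores the off screen.
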(event Custom|RESET_Screens
  (Rendering|SetVisibility (Variables|Default|GetVideoScreen) false false)
  (Rendering|SetVisibility (Variables|Default|GetPanel_9_Big_OFF_Screen) true false))

(event Custom|Toggle%20Video%20To%20Play
  (Media|MediaPlayer|OpenSource (Variables|Default|GetMediaPlayer) "/Game/ART_Spencer/Movies/Videos/Looping_Loading_Background.Looping_Loading_Background"))

(event Custom|Change%20Channel
  (Media|MediaPlayer|OpenSource (Variables|Default|GetMediaPlayer) "/Game/ART_Spencer/Movies/Videos/Looping_Loading_Background.Looping_Loading_Background")
  (Utilities|FlowControl|Delay 0.5)
  (bind _returnvalue (Class|MediaPlaylist|GetRandom (Variables|Default|GetVideo%20Playlist)))
  (Media|MediaPlayer|OpenSource (Variables|Default|GetMediaPlayer) _returnvalue))

(event Custom|Make%20Visible%20Video%20To%20Play
  (Rendering|SetVisibility (Variables|Default|GetPanel_9_Big_OFF_Screen) false false)
  (Rendering|SetVisibility (Variables|Default|GetVideoScreen) true false))

(event Custom|Mute%20Volume
  (Utilities|FlowControl|FlipFlop
    (:A
      (Audio|Components|Audio|SetVolumeMultiplier (Variables|Default|GetMediaSound) 1.0 :!class /Script/AudioMixer.SynthComponent))
    (:B
      (Audio|Components|Audio|SetVolumeMultiplier (Variables|Default|GetMediaSound) 0.0 :!class /Script/AudioMixer.SynthComponent))))

(event EventBeginPlay
  ;[1 1 1] start video muted
  (Audio|Components|Audio|SetVolumeMultiplier (Variables|Default|GetMediaSound) 0.0 :!class /Script/AudioMixer.SynthComponent)
  (CallFunction|MakeVisibleVideotoPlay)
  (CallFunction|ToggleVideotoPlay))

(event Collision|EventActorBeginOverlap
  (params (OtherActor :type Actor%20Object%20Reference)))

(event EventTick
  (params (DeltaSeconds :type Float%20%28single-precision%29)))

(fn ConstructionScript)