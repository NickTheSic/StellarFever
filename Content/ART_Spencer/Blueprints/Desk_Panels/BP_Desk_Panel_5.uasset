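; BP_Desk_Panel_5 is a desk panel prop whose two yellow bulb meshes show whether their panel lights are on.
; Every Tick, it casts two child actor components to BP_Panel_Light_Yellow and polls each one's light visibility.
; Each result sets the matching Panel5Screen mesh to the lit yellow bulb material or the off material, re-applied every frame rather than on change.
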(event EventBeginPlay)

(event Collision|EventActorBeginOverlap
  (params (OtherActor :type Actor%20Object%20Reference)))

(event EventTick
  (params (DeltaSeconds :type Float%20%28single-precision%29))
  (CallFunction|YellowBulbMatChange)
  (CallFunction|YellowBulbMatChange1))

(fn ConstructionScript)

(fn YellowBulbMatChange
  (bind _panel_5_screen023 (Variables|Default|GetPanel_5_Screen023))
  (bind _asbp_panel_light_yellow (Utilities|Casting|CastToBP_Panel_Light_Yellow (Variables|/Script/Engine.ChildActorComponent|GetChildActor (Variables|Default|GetBP_Panel_Light_Yellow))))
  (bind _isvisible (Default|GetLightVisibility _asbp_panel_light_yellow))
  (if _isvisible
    (Rendering|Material|SetMaterial _panel_5_screen023 0 "/Game/ART_Spencer/Blueprints/Desk_Panels/MAT_Yellow_Bulb.MAT_Yellow_Bulb")
    (else
      (Rendering|Material|SetMaterial _panel_5_screen023 0 "/Game/ART_Spencer/Blueprints/Desk_Panels/Mat_Bulb_Off.MAT_Bulb_Off"))))

(fn YellowBulbMatChange1
  (bind _panel_5_screen024 (Variables|Default|GetPanel_5_Screen024))
  (bind _asbp_panel_light_yellow (Utilities|Casting|CastToBP_Panel_Light_Yellow (Variables|/Script/Engine.ChildActorComponent|GetChildActor (Variables|Default|GetBP_Panel_Light_Yellow1))))
  (bind _isvisible (Default|GetLightVisibility _asbp_panel_light_yellow))
  (if _isvisible
    (Rendering|Material|SetMaterial _panel_5_screen024 0 "/Game/ART_Spencer/Blueprints/Desk_Panels/MAT_Yellow_Bulb.MAT_Yellow_Bulb")
    (else
      (Rendering|Material|SetMaterial _panel_5_screen024 0 "/Game/ART_Spencer/Blueprints/Desk_Panels/Mat_Bulb_Off.MAT_Bulb_Off"))))