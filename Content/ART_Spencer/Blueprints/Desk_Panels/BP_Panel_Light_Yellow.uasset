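; Yellow desk panel light actor that blinks its point light on and off at irregular intervals.
; Tick drives a DoOnce that toggles the light's visibility, waits a random delay between RanMin and RanMax, then resets itself to repeat.
; GetLightVisibility stores and returns whether the point light is currently visible.
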(event EventBeginPlay)

(event Collision|EventActorBeginOverlap
  (params (OtherActor :type Actor%20Object%20Reference)))

(event EventTick
  (params (DeltaSeconds :type Float%20%28single-precision%29))
  (Utilities|FlowControl|DoOnce false :!label _label
    (:Completed
      (Rendering|ToggleVisibility (Variables|Default|GetPointLight) false)
      (Utilities|FlowControl|Delay (Math|Random|RandomFloatinRange (Variables|Default|GetRan%20Min) (Variables|Default|GetRan%20Max)))
      (goto _label Reset))))

(fn ConstructionScript)

(fn GetLightVisibility
  (if (Rendering|IsVisible (Variables|Default|GetPointLight))
    (Variables|Default|SetIsLightVisible true)
    (else
      (Variables|Default|SetIsLightVisible false)))
  (return (Variables|Default|GetIsLightVisible)))