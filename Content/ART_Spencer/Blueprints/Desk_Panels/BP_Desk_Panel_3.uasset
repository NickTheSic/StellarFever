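; Desk panel prop whose four indicator bulbs (two green, one red, one yellow) show lit or off materials to match their panel lights.
; Each bulb has a function that casts a child-actor light Blueprint, reads its light visibility and sets the matching screen mesh to a coloured or off material.
; All four functions run every Tick, polling the lights and reapplying materials even when nothing has changed.
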(event EventTick
  (params (DeltaSeconds :type Float%20%28single-precision%29))
  (CallFunction|YellowBulbMatChange)
  (CallFunction|RedBulbMatChange)
  (CallFunction|GreenBulbMatChange)
  (CallFunction|GreenBulbMatChange1))

(event Collision|EventActorBeginOverlap
  (params (OtherActor :type Actor%20Object%20Reference)))

(event EventBeginPlay)

(fn ConstructionScript)

(fn GreenBulbMatChange
  (bind _panel_3_screen025 (Variables|Default|GetPanel_3_Screen025))
  (bind _asbp_panel_light_green (Utilities|Casting|CastToBP_Panel_Light_Green (Variables|/Script/Engine.ChildActorComponent|GetChildActor (Variables|Default|GetBP_Panel_Light_Green))))
  (bind _isvisible (Default|GetLightVisibility _asbp_panel_light_green))
  (if _isvisible
    (Rendering|Material|SetMaterial _panel_3_screen025 0 "/Game/ART_Spencer/Blueprints/Desk_Panels/MAT_Green_Bulb.MAT_Green_Bulb")
    (else
      (Rendering|Material|SetMaterial _panel_3_screen025 0 "/Game/ART_Spencer/Blueprints/Desk_Panels/Mat_Bulb_Off.MAT_Bulb_Off"))))

(fn RedBulbMatChange
  (bind _panel_3_screen026 (Variables|Default|GetPanel_3_Screen026))
  (bind _asbp_panel_light_red (Utilities|Casting|CastToBP_Panel_Light_Red (Variables|/Script/Engine.ChildActorComponent|GetChildActor (Variables|Default|GetBP_Panel_Light_Red))))
  (bind _isvisible (Default|GetLightVisibility _asbp_panel_light_red))
  (if _isvisible
    (Rendering|Material|SetMaterial _panel_3_screen026 0 "/Game/ART_Spencer/Blueprints/Desk_Panels/MAT_Red_Bulb.MAT_Red_Bulb")
    (else
      (Rendering|Material|SetMaterial _panel_3_screen026 0 "/Game/ART_Spencer/Blueprints/Desk_Panels/Mat_Bulb_Off.MAT_Bulb_Off"))))

(fn YellowBulbMatChange
  (bind _panel_3_screen027 (Variables|Default|GetPanel_3_Screen027))
  (bind _asbp_panel_light_yellow (Utilities|Casting|CastToBP_Panel_Light_Yellow (Variables|/Script/Engine.ChildActorComponent|GetChildActor (Variables|Default|GetBP_Panel_Light_Yellow))))
  (bind _isvisible (Default|GetLightVisibility _asbp_panel_light_yellow))
  (if _isvisible
    (Rendering|Material|SetMaterial _panel_3_screen027 0 "/Game/ART_Spencer/Blueprints/Desk_Panels/MAT_Yellow_Bulb.MAT_Yellow_Bulb")
    (else
      (Rendering|Material|SetMaterial _panel_3_screen027 0 "/Game/ART_Spencer/Blueprints/Desk_Panels/Mat_Bulb_Off.MAT_Bulb_Off"))))

(fn GreenBulbMatChange1
  (bind _panel_3_screen028 (Variables|Default|GetPanel_3_Screen028))
  (bind _asbp_panel_light_green (Utilities|Casting|CastToBP_Panel_Light_Green (Variables|/Script/Engine.ChildActorComponent|GetChildActor (Variables|Default|GetBP_Panel_Light_Green1))))
  (bind _isvisible (Default|GetLightVisibility _asbp_panel_light_green))
  (if _isvisible
    (Rendering|Material|SetMaterial _panel_3_screen028 0 "/Game/ART_Spencer/Blueprints/Desk_Panels/MAT_Green_Bulb.MAT_Green_Bulb")
    (else
      (Rendering|Material|SetMaterial _panel_3_screen028 0 "/Game/ART_Spencer/Blueprints/Desk_Panels/Mat_Bulb_Off.MAT_Bulb_Off"))))