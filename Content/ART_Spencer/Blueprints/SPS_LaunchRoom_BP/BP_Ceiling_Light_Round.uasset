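; BP_Ceiling_Light_Round is a round ceiling light that the player switches off and on with the 2 key.
; It enables player input on BeginPlay, and the key drives a FlipFlop that swaps the bulb material between off and lit.
; Both branches toggle visibility on its point light, two child-actor lights and two referenced point light actors, so their state flips relative to the starting visibility.
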(event EventBeginPlay
  ;[1 1 1] for the key press
  (Input|EnableInput (Game|GetPlayerController 0)))

(event Collision|EventActorBeginOverlap
  (params (OtherActor :type Actor%20Object%20Reference)))

(event EventTick
  (params (DeltaSeconds :type Float%20%28single-precision%29)))

(event Input|KeyboardEvents|2
  (params (Key :type Key%20Structure :default "None"))
  (bind _pointlight1 (Variables|Default|GetPointLight1))
  (:Pressed
    (Utilities|FlowControl|FlipFlop
      (:A
        (Rendering|Material|SetMaterial (Variables|Default|Getmesh_bulb) 0 "/Game/ART_Spencer/Blueprints/Desk_Panels/Mat_Bulb_Off.MAT_Bulb_Off")
        (Rendering|ToggleVisibility _pointlight1 false)
        (Rendering|ToggleVisibility (Variables|/Script/Engine.Actor|GetRootComponent (Variables|/Script/Engine.ChildActorComponent|GetChildActor (Variables|Default|GetCeiling_RoundLight_Large))) false)
        (Rendering|ToggleVisibility (Variables|/Script/Engine.Actor|GetRootComponent (Variables|/Script/Engine.ChildActorComponent|GetChildActor (Variables|Default|GetCeiling_RoundLight_Large1))) false)
        (Rendering|ToggleVisibility (Variables|/Script/Engine.Actor|GetRootComponent (Variables|Default|GetAPointLightRef)) false)
        (Rendering|ToggleVisibility (Variables|/Script/Engine.Actor|GetRootComponent (Variables|Default|GetAPointLightRef1)) false))
      (:B
        (Rendering|Material|SetMaterial (Variables|Default|Getmesh_bulb) 0 "/Game/ART_Spencer/Static_Meshes/SPS_Lauch_Room/MAT_Ceiling_Lights_Thin_Bulb.MAT_Ceiling_Lights_Thin_Bulb")
        (Rendering|ToggleVisibility _pointlight1 false)
        (Rendering|ToggleVisibility (Variables|/Script/Engine.Actor|GetRootComponent (Variables|/Script/Engine.ChildActorComponent|GetChildActor (Variables|Default|GetCeiling_RoundLight_Large))) false)
        (Rendering|ToggleVisibility (Variables|/Script/Engine.Actor|GetRootComponent (Variables|/Script/Engine.ChildActorComponent|GetChildActor (Variables|Default|GetCeiling_RoundLight_Large1))) false)
        (Rendering|ToggleVisibility (Variables|/Script/Engine.Actor|GetRootComponent (Variables|Default|GetAPointLightRef)) false)
        (Rendering|ToggleVisibility (Variables|/Script/Engine.Actor|GetRootComponent (Variables|Default|GetAPointLightRef1)) false)))))

(fn ConstructionScript)