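; Launch room big screen actor that swaps an off screen for a media-player video.
; Pressing 3 mutes the media sound, swaps screen visibility, hides the rect light and opens the countdown video.
; Separate events reset the screens, toggle volume via FlipFlop, or change channel by showing a loading loop before opening a random playlist entry.
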(event Custom|RESET_Screens
  (Rendering|SetVisibility (Variables|Default|GetLaunchRoomBigScreen) false false)
  (Rendering|SetVisibility (Variables|Default|GetOff%20Screen) true false))

(event Custom|Toggle%20Video%20To%20Play
  (Media|MediaPlayer|OpenSource (Variables|Default|GetMediaPlayer) "/Game/ART_Spencer/Movies/Videos/SPS_Big_Screen_Countdown.SPS_Big_Screen_Countdown"))

(event Custom|Change%20Channel
  (Media|MediaPlayer|OpenSource (Variables|Default|GetMediaPlayer) "/Game/ART_Spencer/Movies/Videos/Looping_Loading_Background.Looping_Loading_Background")
  (Utilities|FlowControl|Delay 0.5)
  (bind _returnvalue (Class|MediaPlaylist|GetRandom (Variables|Default|GetVideo%20Playlist)))
  (Media|MediaPlayer|OpenSource (Variables|Default|GetMediaPlayer) _returnvalue))

(event Custom|Make%20Visible%20Video%20To%20Play
  (Rendering|SetVisibility (Variables|Default|GetOff%20Screen) false false)
  (Rendering|SetVisibility (Variables|Default|GetLaunchRoomBigScreen) true false)
  (Rendering|SetVisibility (Variables|Default|GetRectLight) false false))

(event Custom|Mute%20Volume
  (Utilities|FlowControl|FlipFlop
    (:A
      (Audio|Components|Audio|SetVolumeMultiplier (Variables|Default|GetMediaSound) 1.0 :!class /Script/AudioMixer.SynthComponent))
    (:B
      (Audio|Components|Audio|SetVolumeMultiplier (Variables|Default|GetMediaSound) 0.0 :!class /Script/AudioMixer.SynthComponent))))

(event EventBeginPlay
  ;[1 1 1] for the key press
  (Input|EnableInput (Game|GetPlayerController 0)))

(event Collision|EventActorBeginOverlap
  (params (OtherActor :type Actor%20Object%20Reference)))

(event EventTick
  (params (DeltaSeconds :type Float%20%28single-precision%29)))

(event Input|KeyboardEvents|3
  (params (Key :type Key%20Structure))
  (:Pressed
    ;[1 1 1] start video muted
    (Audio|Components|Audio|SetVolumeMultiplier (Variables|Default|GetMediaSound) 0.0 :!class /Script/AudioMixer.SynthComponent)
    (CallFunction|MakeVisibleVideotoPlay)
    (CallFunction|ToggleVideotoPlay self)))

(fn ConstructionScript)