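; Long-box plant tank prop that displays small sprouts, large leaf plants, both or neither, based on two boolean flags.
; On BeginPlay it hides all the plant components, then the ShowSmallPlants and ShowLargePlants flags each re-show their group through a matching function.
; The construction script is empty, so the flags only take effect at runtime.
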(event EventBeginPlay
  (CallFunction|HideAllPlants)
  (if (Variables|Default|GetShow_Small_Plants)
    (CallFunction|ShowSmallPlants))
  (if (Variables|Default|GetShow_Large_Plants)
    (CallFunction|ShowLargePlants)))

(event Collision|EventActorBeginOverlap
  (params (OtherActor :type Actor%20Object%20Reference)))

(event EventTick
  (params (DeltaSeconds :type Float%20%28single-precision%29)))

(fn ConstructionScript)

(fn ShowSmallPlants
  (Rendering|SetVisibility (Variables|Default|GetPlants_tanks_and_dirt_SproutSmall6) true false))

(fn HideAllPlants
  (Rendering|SetVisibility (Variables|Default|GetPlants_tanks_and_dirt_LargeLeafPlant02) false false))

(fn ShowLargePlants
  (Rendering|SetVisibility (Variables|Default|GetPlants_tanks_and_dirt_LargeLeafPlant01) true false))