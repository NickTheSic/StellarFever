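; BP_PlantTank_Wall is a plant tank wall prop with three tall leaf plant components that can be shown individually.
; On BeginPlay it hides all three through HideAllPlants, then shows each one whose Plant1, Plant2 or Plant3 flag is set.
; The construction script is empty, so this selection is applied only when play begins, and nothing changes it afterwards.
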(event EventBeginPlay
  (CallFunction|HideAllPlants)
  (if (Variables|Default|GetPlant_1)
    (Rendering|SetVisibility (Variables|Default|GetPlants_tanks_and_dirt_Tall_Leaf_Plant00) true false))
  (if (Variables|Default|GetPlant_2)
    (Rendering|SetVisibility (Variables|Default|GetPlants_tanks_and_dirt_Tall_Leaf_Plant01) true false))
  (if (Variables|Default|GetPlant_3)
    (Rendering|SetVisibility (Variables|Default|GetPlants_tanks_and_dirt_Tall_Leaf_Plant02) true false)))

(event Collision|EventActorBeginOverlap
  (params (OtherActor :type Actor%20Object%20Reference)))

(event EventTick
  (params (DeltaSeconds :type Float%20%28single-precision%29)))

(fn ConstructionScript)

(fn HideAllPlants
  (Rendering|SetVisibility (Variables|Default|GetPlants_tanks_and_dirt_Tall_Leaf_Plant02) false false))