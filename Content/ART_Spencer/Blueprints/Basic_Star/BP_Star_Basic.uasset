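; BP_Star_Basic is a star actor that twinkles by switching its Sphere between normal and dim materials at random intervals.
; Tick feeds two chained Delays, each timed randomly between RandomTimeMin and RandomTimeMax, setting the dim material after the first and the normal one after the second.
; Tick re-arms the first Delay while the second is still pending, so the two timers overlap rather than strictly alternate.
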(event EventBeginPlay)

(event Collision|EventActorBeginOverlap
  (params (OtherActor :type Actor%20Object%20Reference)))

(event EventTick
  (params (DeltaSeconds :type Float%20%28single-precision%29))
  (Utilities|FlowControl|Delay (Math|Random|RandomFloatinRange (Variables|Default|GetRandomTimeMin) (Variables|Default|GetRandomTimeMax)))
  (Rendering|Material|SetMaterial (Variables|Default|GetSphere) 0 "/Game/ART_Spencer/Blueprints/Basic_Star/Mat_Basic_Star_Dim.Mat_Basic_Star_Dim")
  (Utilities|FlowControl|Delay (Math|Random|RandomFloatinRange (Variables|Default|GetRandomTimeMin) (Variables|Default|GetRandomTimeMax)))
  (Rendering|Material|SetMaterial (Variables|Default|GetSphere) 0 "/Game/ART_Spencer/Blueprints/Basic_Star/Mat_Basic_Star.Mat_Basic_Star"))

(fn ConstructionScript)