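; BP_PlantTank_SquareBox is a plant tank prop that shows a configurable selection of plants: two bonsai trees, large and small sprouts, and a large leaf plant.
; On BeginPlay, HideAllPlants hides every plant component, then a separate boolean for each plant makes the chosen ones visible.
; The construction script is empty, so the selection applies only at runtime, and several plants can show at once.
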(event EventBeginPlay
  (CallFunction|HideAllPlants)
  (if (Variables|Default|GetBonsai%201)
    (Rendering|SetVisibility (Variables|Default|GetPlants_tanks_and_dirt_Bonsai_tree_1) true false))
  (if (Variables|Default|GetBonsai%202)
    (Rendering|SetVisibility (Variables|Default|GetPlants_tanks_and_dirt_Bonsai_Tree_2) true false))
  (if (Variables|Default|GetSprout%20Large)
    (Rendering|SetVisibility (Variables|Default|GetPlants_tanks_and_dirt_SproutLarge) true false))
  (if (Variables|Default|GetSprout%20Small)
    (Rendering|SetVisibility (Variables|Default|GetPlants_tanks_and_dirt_SproutSmall) true false))
  (if (Variables|Default|GetLeaf%20Plant%20Large)
    (Rendering|SetVisibility (Variables|Default|GetPlants_tanks_and_dirt_LargeLeafPlant01) true false)))

(event Collision|EventActorBeginOverlap
  (params (OtherActor :type Actor%20Object%20Reference)))

(event EventTick
  (params (DeltaSeconds :type Float%20%28single-precision%29)))

(fn ConstructionScript)

(fn HideAllPlants
  (Rendering|SetVisibility (Variables|Default|GetPlants_tanks_and_dirt_SproutLarge) false false))