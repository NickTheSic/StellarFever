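; BP_AudioLog is an interactable audio log that plays its assigned sound when the player presses E inside its trigger box.
; Box overlap begin and end enable and disable input, and a DoOnce limits playback to a single use through the audio component.
; Tick blinks the on-light using a DoOnce reset after a short delay, then shows only the off-light once HasBeenUsed is set.
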(event OnComponentBeginOverlap(BoxTrigger)
  (params (OverlappedComponent :type Primitive%20Component%20Object%20Reference) (OtherActor :type Actor%20Object%20Reference) (OtherComp :type Primitive%20Component%20Object%20Reference) (OtherBodyIndex :type Integer) (bFromSweep :type Boolean) (SweepResult :type Hit%20Result%20Structure%20%28by%20ref%29))
  ;[1 1 1] Input Enabler
  (Input|EnableInput (Game|GetPlayerController 0)))

(event OnComponentEndOverlap(BoxTrigger)
  (params (OverlappedComponent :type Primitive%20Component%20Object%20Reference) (OtherActor :type Actor%20Object%20Reference) (OtherComp :type Primitive%20Component%20Object%20Reference) (OtherBodyIndex :type Integer))
  ;[1 1 1] Input Enabler
  (Input|DisableInput (Game|GetPlayerController 0)))

(event EventTick
  (params (DeltaSeconds :type Float%20%28single-precision%29))
  (if (Variables|Default|GetHasBeenUsed)
    (Rendering|SetVisibility (Variables|Default|GetOn_Light) false false)
    (Rendering|SetVisibility (Variables|Default|GetOff_Light) true false)
    (else
      ;[1 1 1] to prevent flicker on button press
      (Utilities|FlowControl|DoOnce false :!label _label
        (:Completed
          (Rendering|ToggleVisibility (Variables|Default|GetOn_Light) false)
          (Utilities|FlowControl|Delay 0.5)
          (goto _label Reset))))))

(event Input|KeyboardEvents|E
  (params (Key :type Key%20Structure))
  (:Pressed
    (Utilities|FlowControl|DoOnce (Variables|Default|GetHasBeenUsed)
      (:Completed
        (Variables|Default|SetHasBeenUsed true)
        (Audio|Components|Audio|SetSound (Variables|Default|GetAudioComponentToPlay) (Variables|Default|GetSoundBase))
        (Audio|Components|Audio|Play (Variables|Default|GetAudioComponentToPlay) 0.0)))))

(fn ConstructionScript)