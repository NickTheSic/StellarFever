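; BP_HallwayCables is a hallway cable set piece with optional spark effects at its start or end.
; On BeginPlay, two toggles pick the active Sparks reference, with the end taking priority, and move the actor to that component's attach-parent world location.
; Tick and the construction script are empty, and a ToggleActive call on Sparks is left unconnected.
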(event EventBeginPlay
  (bind _sparks1 (Variables|Default|GetSparks1))
  (if (Variables|Default|GetSparksEndToggle)
    (Variables|Default|SetSparks _sparks1)
    (Transformation|SetActorLocation (Transformation|GetWorldLocation (Transformation|GetAttachParent _sparks1)) false false)
    (elif (Variables|Default|GetSparksStartToggle)
      (Variables|Default|SetSparks (Variables|Default|GetSparks))
      (Transformation|SetActorLocation (Transformation|GetWorldLocation (Transformation|GetAttachParent (Variables|Default|GetSparks))) false false))))

(event Collision|EventActorBeginOverlap
  (params (OtherActor :type Actor%20Object%20Reference)))

(event EventTick
  (params (DeltaSeconds :type Float%20%28single-precision%29)))

(fn ConstructionScript)