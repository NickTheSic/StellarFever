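; BP_PosterDecal is a poster decal Blueprint with four tape components whose visibility is controlled by boolean options.
; On BeginPlay, it hides each of Tape1, Tape2 and Tape3 whose matching TapeON flag is false.
; The first Tape works differently: only if it starts invisible is its visibility set to TapeON, so that flag never hides it.
; The construction script is empty, so these options apply only at runtime.
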(event EventBeginPlay
  (if (Rendering|IsVisible (Variables|Default|GetTape))
    _
    (else
      (Rendering|SetVisibility (Variables|Default|GetTape) (Variables|Default|GetTapeON) false)))
  (if (Variables|Default|GetTapeON1)
    _
    (else
      (Rendering|SetVisibility (Variables|Default|GetTape1) false false)))
  (if (Variables|Default|GetTapeON2)
    _
    (else
      (Rendering|SetVisibility (Variables|Default|GetTape2) false false)))
  (if (not (Variables|Default|GetTapeON3))
    (Rendering|SetVisibility (Variables|Default|GetTape3) false false)))

(fn ConstructionScript)