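; BP_RoomDoor is an automatic room door that opens when a Character enters its Box trigger and closes when the last one leaves.
; A NumInteracted counter tracks overlapping Characters, so only the first entry and last exit drive the skeletal mesh's separate open and close animations.
; If an animation is still playing at that moment, its play rate is negated to reverse the door mid-motion instead of starting another animation.
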(event OnComponentBeginOverlap(Box)
  (params (OverlappedComponent :type Primitive%20Component%20Object%20Reference) (OtherActor :type Actor%20Object%20Reference) (OtherComp :type Primitive%20Component%20Object%20Reference) (OtherBodyIndex :type Integer) (bFromSweep :type Boolean) (SweepResult :type Hit%20Result%20Structure%20%28by%20ref%29))
  (bind _skeletalmesh (Variables|Default|GetSkeletalMesh))
  ;[1 1 1] Open Door Animation
  (Utilities|Casting|CastToCharacter OtherActor)
  (Variables|Default|SetnumInteracted (+ (Variables|Default|GetnumInteracted) 1))
  (if (== (Variables|Default|GetnumInteracted) 1)
    (if (Audio|Components|Audio|IsPlaying _skeletalmesh)
      (Components|Timeline|SetPlayRate _skeletalmesh (* (Components|Animation|GetPlayRate _skeletalmesh) -1.0))
      (else
        (Components|Animation|PlayAnimation _skeletalmesh "/Game/Kentyn_Models/Doors/Room_Door/ANM_Room_Door_Open.ANM_Room_Door_Open" false)
        (Components|Timeline|SetPlayRate _skeletalmesh 2.5)))))

(event OnComponentEndOverlap(Box)
  (params (OverlappedComponent :type Primitive%20Component%20Object%20Reference) (OtherActor :type Actor%20Object%20Reference) (OtherComp :type Primitive%20Component%20Object%20Reference) (OtherBodyIndex :type Integer))
  (bind _skeletalmesh (Variables|Default|GetSkeletalMesh))
  ;[1 1 1] Close Door Animation
  (Utilities|Casting|CastToCharacter OtherActor)
  (Variables|Default|SetnumInteracted (- (Variables|Default|GetnumInteracted) 1))
  (if (== (Variables|Default|GetnumInteracted) 0)
    (if (Audio|Components|Audio|IsPlaying _skeletalmesh)
      (Components|Timeline|SetPlayRate _skeletalmesh (* (Components|Animation|GetPlayRate _skeletalmesh) -1.0))
      (else
        (Components|Animation|PlayAnimation _skeletalmesh "/Game/Kentyn_Models/Doors/Room_Door/ANM_Room_DoorOpenClose.ANM_Room_DoorOpenClose" false)
        (Components|Timeline|SetPlayRate _skeletalmesh 2.5)))))

(event EventBeginPlay)

(event Collision|EventActorBeginOverlap
  (params (OtherActor :type Actor%20Object%20Reference)))

(event EventTick
  (params (DeltaSeconds :type Float%20%28single-precision%29)))

(fn ConstructionScript)