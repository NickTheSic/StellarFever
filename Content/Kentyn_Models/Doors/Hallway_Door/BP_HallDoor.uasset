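; BP_HallDoor is an automatic animated door that opens when Characters enter its trigger box and closes once all have left.
; An overlap counter fires the animations only for the first Character in and the last one out.
; If the skeletal mesh is still animating, its play rate is negated to reverse the motion midway.
; An "Airlock" actor tag swaps in the airlock animations at a faster play rate.
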(event OnComponentBeginOverlap(Box)
  (params (OverlappedComponent :type Primitive%20Component%20Object%20Reference) (OtherActor :type Actor%20Object%20Reference) (OtherComp :type Primitive%20Component%20Object%20Reference) (OtherBodyIndex :type Integer) (bFromSweep :type Boolean) (SweepResult :type Hit%20Result%20Structure%20%28by%20ref%29))
  (bind _returnvalue (Actor|ActorHasTag "Airlock"))
  (bind _skeletalmesh (Variables|Default|GetSkeletalMesh))
  (bind _returnvalue_2 (not _returnvalue))
  (bind _returnvalue_3 (Components|Animation|GetPlayRate _skeletalmesh))
  (bind _returnvalue_4 (* _returnvalue_3 -1.0))
  ;[1 1 1] Open Door Animation
  (Utilities|Casting|CastToCharacter OtherActor)
  (Variables|Default|SetnumInteracted (+ (Variables|Default|GetnumInteracted) 1))
  (if (== (Variables|Default|GetnumInteracted) 1)
    (if (Audio|Components|Audio|IsPlaying _skeletalmesh)
      (if _returnvalue_2
        (Components|Timeline|SetPlayRate _skeletalmesh _returnvalue_4)
        (else
          (Components|Timeline|SetPlayRate _skeletalmesh _returnvalue_4)))
      (elif _returnvalue_2
        (Components|Animation|PlayAnimation _skeletalmesh "/Game/Kentyn_Models/Doors/Hallway_Door/ANM_Hallway_Door_Open.ANM_Hallway_Door_Open" false)
        (Components|Timeline|SetPlayRate _skeletalmesh 2.5)
        (else
          (Components|Animation|PlayAnimation _skeletalmesh "/Game/ART_Spencer/Static_Meshes/Airlock_Props/Airlock_Door/Airlock_Door_Open.Airlock_Door_Open" false)
          (Components|Timeline|SetPlayRate _skeletalmesh 3.5))))))

(event OnComponentEndOverlap(Box)
  (params (OverlappedComponent :type Primitive%20Component%20Object%20Reference) (OtherActor :type Actor%20Object%20Reference) (OtherComp :type Primitive%20Component%20Object%20Reference) (OtherBodyIndex :type Integer))
  (bind _returnvalue (Actor|ActorHasTag "Airlock"))
  (bind _skeletalmesh (Variables|Default|GetSkeletalMesh))
  (bind _returnvalue_2 (not _returnvalue))
  (bind _returnvalue_3 (Components|Animation|GetPlayRate _skeletalmesh))
  (bind _returnvalue_4 (* _returnvalue_3 -1.0))
  ;[1 1 1] Close Door Animation
  (Utilities|Casting|CastToCharacter OtherActor)
  (Variables|Default|SetnumInteracted (- (Variables|Default|GetnumInteracted) 1))
  (if (== (Variables|Default|GetnumInteracted) 0)
    (if (Audio|Components|Audio|IsPlaying _skeletalmesh)
      (if _returnvalue_2
        (Components|Timeline|SetPlayRate _skeletalmesh _returnvalue_4)
        (else
          (Components|Timeline|SetPlayRate _skeletalmesh _returnvalue_4)))
      (elif _returnvalue_2
        (Components|Animation|PlayAnimation _skeletalmesh "/Game/Kentyn_Models/Doors/Hallway_Door/ANM_Hallway_Door_Close.ANM_Hallway_Door_Close" false)
        (Components|Timeline|SetPlayRate _skeletalmesh 2.5)
        (else
          (Components|Animation|PlayAnimation _skeletalmesh "/Game/ART_Spencer/Static_Meshes/Airlock_Props/Airlock_Door/Airlock_Door_Close.Airlock_Door_Close" false)
          (Components|Timeline|SetPlayRate _skeletalmesh 3.5))))))

(event EventBeginPlay)

(event Collision|EventActorBeginOverlap
  (params (OtherActor :type Actor%20Object%20Reference)))

(event EventTick
  (params (DeltaSeconds :type Float%20%28single-precision%29)))

(fn ConstructionScript)