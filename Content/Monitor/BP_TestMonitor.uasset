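; BP_TestMonitor is a wrapper actor that configures a BP_TV_Info_Monitor child actor with a chosen stand type.
; On BeginPlay it copies its base, jetpack, wheels, propeller and wall arm flags to the child, then calls ShowCorrectStands.
; With jetpack or propeller set, it stores its start location and bobs vertically around it each Tick using a cosine of game time.
; A leftover chain that clears the child's flags never runs.
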(event EventBeginPlay
  (bind _asbp_tv_info_monitor (Utilities|Casting|CastToBP_TV_Info_Monitor (Variables|/Script/Engine.ChildActorComponent|GetChildActor (Variables|Default|GetpModel))))
  (Variables|/Game/ART_Spencer/Blueprints/BP_TV_Info_Monitor.BP_TV_Info_Monitor_C|SetBasic_Base _asbp_tv_info_monitor (Variables|Default|GetBase))
  (Variables|/Game/ART_Spencer/Blueprints/BP_TV_Info_Monitor.BP_TV_Info_Monitor_C|SetJet_Pack _asbp_tv_info_monitor (Variables|Default|GetJetpack))
  (Variables|/Game/ART_Spencer/Blueprints/BP_TV_Info_Monitor.BP_TV_Info_Monitor_C|SetWheel_Base _asbp_tv_info_monitor (Variables|Default|GetWheels))
  (Variables|/Game/ART_Spencer/Blueprints/BP_TV_Info_Monitor.BP_TV_Info_Monitor_C|SetPropeller _asbp_tv_info_monitor (Variables|Default|GetPropeller))
  (Variables|/Game/ART_Spencer/Blueprints/BP_TV_Info_Monitor.BP_TV_Info_Monitor_C|SetWall_Arm_1 _asbp_tv_info_monitor (Variables|Default|GetArm%201))
  (Variables|/Game/ART_Spencer/Blueprints/BP_TV_Info_Monitor.BP_TV_Info_Monitor_C|SetWall_Arm_2 _asbp_tv_info_monitor (Variables|Default|GetArm%202))
  (Default|ShowCorrectStands _asbp_tv_info_monitor)
  (if (or (Variables|Default|GetJetpack) (Variables|Default|GetPropeller))
    (bind _output_get (Variables|Default|SetMagic (Transformation|GetActorLocation)))))

(event EventTick
  (params (DeltaSeconds :type Float%20%28single-precision%29))
  (if (or (Variables|Default|GetJetpack) (Variables|Default|GetPropeller))
    (Transformation|SetActorLocation (+ (stale EventBeginPlay _output_get) (Math|Vector|MakeVector 0.0 0.0 (* (* (Math|Trig|Cos(Radians) (Utilities|Time|GetGameTimeinSeconds)) 2.0) 5.0))) false false)))

(fn ConstructionScript)