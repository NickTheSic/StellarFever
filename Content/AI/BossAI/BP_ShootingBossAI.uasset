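; Shooting boss AI actor that, as wired, only drives its boss health bar widget.
; Tick pushes health values to the widget and hides it when player 0 is beyond a set distance.
; ServerGrenadeShot calls an empty GrenadeShot, and its looping timer is disconnected.
; Disconnected GrenadeShot drafts target the nearest or blackboard player, solving the ballistic equation for the lower launch pitch to spawn frag grenades.
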(event Custom|ServerGrenadeShot
  (CallFunction|GrenadeShot))

(event EventBeginPlay)

(event EventTick
  (params (DeltaSeconds :type Float%20%28single-precision%29))
  (bind _phealthcomp (Variables|Default|GetpHealthComp))
  (Utilities|FlowControl|Sequence
    (:then_0
      (bind _aswbp_boss_health (Utilities|Casting|CastToWBP_BossHealth (UserInterface|GetUserWidgetObject (Variables|Default|GetBossHealthWidget))))
      (bind _output_get (Variables|Default|SetBossHealthBarWidget _aswbp_boss_health))
      (Default|UpdateHealth _output_get (Variables|/Script/StellarFever.HealthComponent|GetHealth _phealthcomp) (Variables|/Script/StellarFever.HealthComponent|GetDefaultHealth _phealthcomp)))
    (:then_1
      (if (> (Transformation|GetDistanceTo (Game|Player|GetPlayerPawn 0)) 3.2e+03)
        (Variables|/Game/AI/UI/WBP_BossHealth.WBP_BossHealth_C|SetHide (Variables|Default|GetBossHealthBarWidget) true)
        (else
          (Variables|/Game/AI/UI/WBP_BossHealth.WBP_BossHealth_C|SetHide (Variables|Default|GetBossHealthBarWidget) false))))))

(fn ConstructionScript)

(fn GrenadeShot
  ;[1 1 1] OLD 1
)